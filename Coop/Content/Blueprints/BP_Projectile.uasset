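; BP_Projectile is a timed explosive projectile that detonates one second after it spawns.
; On BeginPlay a delay leads into the Explode event, which spawns an explosion particle effect and applies full, non-falloff radial damage credited to the instigator.
; It also draws a brief red debug sphere showing the damage radius.
; The graph contains no impact handling or self-destruction after the blast.
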(event Custom|Explode
  (bind _returnvalue (Transformation|GetActorLocation))
  (Effects|SpawnEmitteratLocation "/Game/WeaponEffects/Explosion/P_Explosion.P_Explosion" _returnvalue)
  (Game|Damage|ApplyRadialDamage 1e+02 _returnvalue (Variables|Default|GetDmgRadius) 0 0 self (Game|GetInstigatorController) true "ECC_Visibility")
  (Rendering|Debug|DrawDebugSphere _returnvalue (Variables|Default|GetDmgRadius) 12 "(R=1.000000,G=0.046875,B=0.046875,A=1.000000)" 0.5 2.0))

(event EventBeginPlay
  (Utilities|FlowControl|Delay 1.0)
  (CallFunction|Explode))

(fn ConstructionScript)